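; OpenDoor_BP is an interactive double door that opens and closes on the E key while the input is enabled by its Trigger volume.
; Trigger overlap begin and end enable and disable input for player controller 0, without checking which actor overlaps.
; E-key handlers check each timeline's current value to play or reverse it, driving the relative yaw of the Left and Right components.
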(event OnComponentBeginOverlap(Trigger)
  (params (OverlappedComponent :type Primitive%20Component%20Object%20Reference) (OtherActor :type Actor%20Object%20Reference) (OtherComp :type Primitive%20Component%20Object%20Reference) (OtherBodyIndex :type Integer) (bFromSweep :type Boolean) (SweepResult :type Hit%20Result%20Structure%20%28by%20ref%29))
  (Input|EnableInput (Game|GetPlayerController 0)))

(event OnComponentEndOverlap(Trigger)
  (params (OverlappedComponent :type Primitive%20Component%20Object%20Reference) (OtherActor :type Actor%20Object%20Reference) (OtherComp :type Primitive%20Component%20Object%20Reference) (OtherBodyIndex :type Integer))
  (Input|DisableInput (Game|GetPlayerController 0)))

(event EventBeginPlay)

(event Collision|EventActorBeginOverlap
  (params (OtherActor :type Actor%20Object%20Reference)))

(event EventTick
  (params (DeltaSeconds :type Float%20%28single-precision%29)))

(event Input|KeyboardEvents|E
  (params (Key :type Key%20Structure :default "None"))
  (:Pressed
    (if (< (stale _leftdoor) -179.990005)
      (bind _leftdoor (Timeline|LeftDoor Play)
        (:Update
          (Transformation|SetRelativeRotation (Variables|Default|GetLeft) (Math|Rotator|MakeRotator 0.0 0.0 _leftdoor) false false)))
      (else
        (Timeline|LeftDoor Reverse)))))

(event Input|KeyboardEvents|E
  (params (Key :type Key%20Structure :default "None"))
  (:Pressed
    (if (> (stale _rightdoor) -0.01)
      (bind _rightdoor (Timeline|RightDoor Play)
        (:Update
          (Transformation|SetRelativeRotation (Variables|Default|GetRight) (Math|Rotator|MakeRotator 0.0 0.0 _rightdoor) false false)))
      (else
        (Timeline|RightDoor Reverse)))))

(fn ConstructionScript)